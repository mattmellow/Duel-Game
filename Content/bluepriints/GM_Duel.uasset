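; GM_Duel is the game mode for a samurai quick-draw duel between a player and an NPC.
; Tick moves the phase from Intro to Wait, then after a random delay to Draw, broadcasting the draw start and showing an exclamation mark.
; A successful attack defeats the other samurai, hides the mark and starts a restart timer.
; Reset restores the Intro phase and both duelists, while a separate function sets Finish.
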(event EventBeginPlay
  (bind _returnvalue (Actor|GetActorOfClass "/Game/bluepriints/BP_exclamation.BP_exclamation_C"))
  (Variables|Default|SetExclamationRef _returnvalue)
  (bind _returnvalue_2 (Actor|GetActorOfClass "/Game/bluepriints/BP_Samurai_Player.BP_Samurai_Player_C"))
  (Variables|Default|Setsamurai%20player _returnvalue_2)
  (bind _returnvalue_3 (Actor|GetActorOfClass "/Game/bluepriints/BP_Samurai_NPC.BP_Samurai_NPC_C"))
  (Variables|Default|Setsamurai%20npc _returnvalue_3))

(event EventTick
  (params (DeltaSeconds :type Float%20%28single-precision%29))
  (Variables|Default|SetElapsedTime (+ DeltaSeconds (Variables|Default|GetElapsedTime)))
  (switch Utilities|FlowControl|Switch|SwitchonE_phase (Variables|Default|GetPhase)
    (:NewEnumerator0
      (if (>= (Variables|Default|GetElapsedTime) (Variables|Default|GetRoundStartTime))
        (Variables|Default|SetPhase "NewEnumerator1")
        (Utilities|FlowControl|Delay (Math|Random|RandomFloatinRange (Variables|Default|GetMin%20draw%20delay) (Variables|Default|GetMax%20draw%20delay)))
        (Variables|Default|SetPhase "NewEnumerator2")
        (Default|CallDrawphasestarted)
        (Utilities|IsValid (Variables|Default|GetExclamationRef)
          (:Is%20Valid
            (Default|SetVisibility (Variables|Default|GetExclamationRef) true))
          (:Is%20Not%20Valid
            (Development|PrintString "not valid")))))))

(fn ConstructionScript)

(fn Setgamefinished
  (Variables|Default|SetPhase "NewEnumerator3"))

(fn Attackedsuccessfully
  (params (isplayer? :type Boolean))
  (if isplayer?
    (Default|Defeat (Variables|Default|Getsamurai%20npc))
    (else
      (Default|Defeat (Variables|Default|Getsamurai%20player))))
  (Utilities|IsValid (Variables|Default|GetExclamationRef)
    (:Is%20Valid
      (Default|SetVisibility (Variables|Default|GetExclamationRef) false)
      (Utilities|Time|SetTimerbyEvent (EventDispatchers|CreateEvent :!event Reset) (Variables|Default|Getrestart%20timer)))))

(fn Reset
  (Variables|Default|SetPhase "NewEnumerator0")
  (Variables|Default|SetElapsedTime 0.0)
  (Default|Reset (Variables|Default|Getsamurai%20player))
  (Default|Reset (Variables|Default|Getsamurai%20npc)))